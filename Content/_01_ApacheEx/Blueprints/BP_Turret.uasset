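; Anti-aircraft truck turret that tracks and shells the player's Apache helicopter.
; Each Tick, unless destroyed or the Apache's IsPopUp is set, it aims the pitch-clamped gun within SearchRange and fires twin BP_TurretRocket within FireRange on a delay cooldown.
; Construction randomly toes the two muzzles apart or together for spread.
; An ApacheRocket overlap fractures gun and truck via radius damage, increments the Apache's kill count, then destroys the actor.
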(event `self.Trigger.OnComponentBeginOverlap`
  (params (OverlappedComponent :type "PrimitiveComponent Object Reference") (OtherActor :type "Actor Object Reference") (OtherComp :type "PrimitiveComponent Object Reference") (OtherBodyIndex :type Integer) (bFromSweep :type Boolean) (SweepResult :type "HitResult Structure (by ref)"))
  (bind _turret_gun_dm (`self.Turret_Gun_DM`))
  (bind _turret_truck_dm (`self.Turret_Truck_DM`))
  ;[1 1 1] 아파치 로켓이 부딪쳤을 때 대공포 파괴
  (if (`self.ActorHasTag` OtherActor "ApacheRocket")
    (`/Engine/EditorBlueprintResources/StandardMacros.DoOnce` false
      (:`Completed`
        (`KismetSystemLibrary.PrintString` "Overlap ApacheRocket")
        (`DestructibleComponent.ApplyRadiusDamage` _turret_gun_dm 100.0 (`SceneComponent.K2_GetComponentLocation` _turret_gun_dm) 100.0 100.0 false)
        (`DestructibleComponent.ApplyRadiusDamage` _turret_truck_dm 100.0 (`SceneComponent.K2_GetComponentLocation` _turret_truck_dm) 100.0 100.0 false)
        (set `self.IsDestroyed` true)
        (`self.SetKillCount`)
        (`KismetSystemLibrary.Delay` 3.0)
        (`self.K2_DestroyActor`)))))

(event `self.ReceiveTick`
  (params (DeltaSeconds :type "Float (single-precision)"))
  ;[1 1 1] 거리 계산 -> 포탑 회전 ->  사격거리판단 -> 포탄발사
  (bind _ispopup (`self.CheckApache`))
  (if (not (or _ispopup (`self.IsDestroyed`)))
    (`self.거리 계산`)
    (`self.포탑 회전`)
    (bind `_포탄발사여부` (`self.사격거리판단`))
    (if `_포탄발사여부`
      (`self.포탄 발사`))))

(event `포탄 발사`
  ;[1 1 1] 포탄 발사 이벤트 처리
  (if (`self.CanFire`)
    (set `self.CanFire` false)
    (`|SpawnActorFromClass` "/Game/_01_ApacheEx/Blueprints/BP_TurretRocket.BP_TurretRocket_C" (`SceneComponent.K2_GetComponentToWorld` (`self.SpawnRight`)) "Undefined" "OverrideRootScale" null null)
    (`|SpawnActorFromClass` "/Game/_01_ApacheEx/Blueprints/BP_TurretRocket.BP_TurretRocket_C" (`SceneComponent.K2_GetComponentToWorld` (`self.SpawnLeft`)) "Undefined" "OverrideRootScale" null null)
    (`KismetSystemLibrary.Delay` (`self.DelayTime`))
    (set `self.CanFire` true)))

(event `거리 계산`
  (bind _returnvalue (`GameplayStatics.GetPlayerPawn` 0))
  ;[1 1 1] 거리 계산 이벤트 처리
  (set `self.TargetRotation` (`KismetMathLibrary.FindLookAtRotation` (`SceneComponent.K2_GetComponentLocation` (`self.Turret_Gun_DM`)) (`self.K2_GetActorLocation` _returnvalue))) ; Gun이 아파치를 향하는 방향
  (set `self.TargetDist` (`self.GetDistanceTo` _returnvalue)) ; Turret액터와 아파치의 거리
)

(event `포탑 회전`
  ;[1 1 1] 포탑 회전 이벤트 처리
  (if (<= (`self.TargetDist`) (`self.SearchRange`))
    (`SceneComponent.K2_SetWorldRotation` (`self.Turret_Gun_DM`) (`KismetMathLibrary.MakeRotator` 0.0 (`KismetMathLibrary.FClamp` (.pitch (`self.TargetRotation`)) 0.0 40.0) (.yaw (`self.TargetRotation`))) false false)))

(fn `CheckApache`
  (returns (IsPopUp :type Boolean))
  (bind _asbp_apache (cast `/Game/_01_ApacheEx/Blueprints/BP_Apache` (`GameplayStatics.GetPlayerPawn` 0)))
  (if (`/Game/_01_ApacheEx/Blueprints/BP_Apache.IsDead` _asbp_apache)
    (set `self.CanFire` false))
  (return (`/Game/_01_ApacheEx/Blueprints/BP_Apache.IsPopUp` _asbp_apache)))

(fn `SetKillCount`
  (bind _asbp_apache (cast `/Game/_01_ApacheEx/Blueprints/BP_Apache` (`GameplayStatics.GetPlayerPawn` 0)))
  (`/Engine/EditorBlueprintResources/StandardMacros.IncrementInt` (`/Game/_01_ApacheEx/Blueprints/BP_Apache.KillCount` _asbp_apache)
    (:`  `
      (`/Game/_01_ApacheEx/Blueprints/BP_Apache.KillCountEvent` _asbp_apache))))

(fn `UserConstructionScript`
  (bind _returnvalue (`KismetMathLibrary.RandomFloatInRange` 0.5 1.2))
  (`SceneComponent.K2_SetRelativeRotation` (`self.SpawnLeft`) (`KismetMathLibrary.MakeRotator` 0.0 0.0 _returnvalue) false false)
  (`SceneComponent.K2_SetRelativeRotation` (`self.SpawnRight`) (`KismetMathLibrary.MakeRotator` 0.0 0.0 (* _returnvalue -1.0)) false false))

(fn `사격거리판단`
  (returns (`포탄발사여부` :type Boolean))
  (return (<= (`self.TargetDist`) (`self.FireRange`))))