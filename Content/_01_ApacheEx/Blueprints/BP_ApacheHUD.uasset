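; HUD Blueprint for the Apache example that draws a horizontally centered material image and text line on screen.
; Each DrawHUD call stores the screen size, then draws HudMaterial and ViewText in ApacheFont at fixed heights.
; GetCenterPos computes the X offset from screen and element width, with text width measured through GetTextSize so any string stays centered.
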(event `self.ReceiveDrawHUD`
  (params (SizeX :type Integer) (SizeY :type Integer))
  (`self.SetScreenSize` SizeX SizeY)
  (`self.DrawCenterMaterial` 500.0 100.0 400.0)
  (`self.DrawCenterText` (`self.ViewText`) (struct :`R` 0.984375 :`G` 0.984141 :`B` 0.95874 :`A` 1.0) 300.0 "/Game/_01_ApacheEx/Fonts/ApacheFont.ApacheFont" 2.0))

(fn `DrawCenterMaterial`
  (params (ImageWidth :type "Float (double-precision)") (ImageHeight :type "Float (double-precision)") (ImageY :type "Float (double-precision)"))
  (bind _centerpos (`self.GetCenterPos` ImageWidth)) ; 머티리얼 이미지의 시작 위치(중심)
  (`self.DrawMaterial` (`self.HudMaterial`) _centerpos ImageY ImageWidth ImageHeight 0.0 0.0 1.0 1.0))

(fn `DrawCenterText`
  (params (ViewText :type String) (TextColor :type "LinearColor Structure") (ScreenY :type "Float (double-precision)") (TextFont :type "Font Object Reference") (Scale :type "Float (double-precision)"))
  (bind _centerpos (`self.GetCenterPos` (`self.GetTextSize` ViewText TextFont Scale)))
  (`self.DrawText` ViewText TextColor _centerpos ScreenY TextFont Scale))

(fn `GetCenterPos`
  (params (Width :type "Float (double-precision)"))
  (returns (CenterPos :type "Float (double-precision)"))
  (return (/ (- (`self.ScreenWidth`) Width) 2.0)))

(fn `SetScreenSize`
  (params (Width :type Integer) (Height :type Integer))
  (set `self.ScreenWidth` (`KismetMathLibrary.Conv_IntToDouble` Width))
  (set `self.ScreenHeight` (`KismetMathLibrary.Conv_IntToDouble` Height)))

(fn `UserConstructionScript`)