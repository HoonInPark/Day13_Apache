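; BP_PickUp is a fuel pickup actor that the Apache collects by touching it.
; When an actor tagged Apache overlaps its static mesh, a DoOnce gate lets it call AddFuel on BP_Apache a single time.
; It then spawns a heal particle effect and plays a pickup sound at its location.
; After a short delay it destroys the emitter and itself.
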(event `self.StaticMesh.OnComponentBeginOverlap`
  (params (OverlappedComponent :type "PrimitiveComponent Object Reference") (OtherActor :type "Actor Object Reference") (OtherComp :type "PrimitiveComponent Object Reference") (OtherBodyIndex :type Integer) (bFromSweep :type Boolean) (SweepResult :type "HitResult Structure (by ref)"))
  (bind _returnvalue (`self.K2_GetActorLocation`))
  (if (`self.ActorHasTag` OtherActor "Apache")
    (`/Engine/EditorBlueprintResources/StandardMacros.DoOnce` false
      (:`Completed`
        (bind _asbp_apache (cast `/Game/_01_ApacheEx/Blueprints/BP_Apache` OtherActor))
        (`/Game/_01_ApacheEx/Blueprints/BP_Apache.AddFuel` _asbp_apache)
        (bind _returnvalue_2 (`GameplayStatics.SpawnEmitterAtLocation` "/Game/InfinityBladeEffects/Effects/FX_Monsters/FX_Monster_Ausar/P_AU_Heal_01.P_AU_Heal_01" _returnvalue (struct) (3.0 3.0 3.0)))
        (`GameplayStatics.PlaySoundAtLocation` "/Game/_01_ApacheEx/Audio/PickupSound.PickupSound" _returnvalue (struct) 1.0 1.0 0.0 null null null)
        (`KismetSystemLibrary.Delay` 1.0)
        (`ActorComponent.K2_DestroyComponent` _returnvalue_2)
        (`self.K2_DestroyActor`)))))

(fn `UserConstructionScript`)