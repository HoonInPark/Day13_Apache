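; Player-controlled Apache helicopter that fights turrets and owns the game's HUD, cockpit and menu widgets.
; Input axes drive FInterpTo-smoothed movement and yaw, with turning also rolling the SpringArm; a toggle switches cockpit and third-person views.
; Fire press and release launch left and right rockets.
; Tick drains fuel, derives HP from it and checks kill count; completion, empty fuel or a turret rocket hit opens the main menu.
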(event `InputAxis|앞뒤이동`
  (params (AxisValue :type "Float (single-precision)"))
  ;[1 1 1] 앞뒤 선형보간 이동 기능
  (bind _returncurrent (`self.선형보간` (`self.CurrentX`) AxisValue (`self.SpeedMove`)))
  (bind _output_get (set `self.CurrentX` _returncurrent))
  (`self.K2_AddActorLocalOffset` (`KismetMathLibrary.MakeVector` _output_get) true))

(event `InputAxis|좌우이동`
  (params (AxisValue :type "Float (single-precision)"))
  ;[1 1 1] 좌우 선형보간 이동 기능
  (bind _returncurrent (`self.선형보간` (`self.CurrentY`) AxisValue (`self.SpeedMove`)))
  (bind _output_get (set `self.CurrentY` _returncurrent))
  (`self.K2_AddActorLocalOffset` (`KismetMathLibrary.MakeVector` 0.0 _output_get) true))

(event `MouseLeftRightEvent`
  (params (`Axis Value` :type "Float (double-precision)"))
  ;[1 1 1] 좌우 선형보간 회전 기능
  (`|ExecutionSequence`
    (:`then_0`
      (bind _returncurrent (`self.선형보간` (`self.CurrentYaw`) `Axis Value` (* (`self.SpeedRot`) 2.0)))
      (bind _output_get (set `self.CurrentYaw` _returncurrent))
      (`self.K2_AddActorLocalRotation` (`KismetMathLibrary.MakeRotator` 0.0 0.0 _output_get) true))
    (:`then_1`
      ;[1 1 1] 키보드와 마우스 회전 적용
      ;;[1 1 1] 회전시 SpringArm을 반대로 기울이기 값을 저장한다
      (bind _returncurrent_2 (`self.선형보간` (`self.ArmRoll`) `Axis Value` (`self.SpeedRoll`)))
      (set `self.ArmRoll` _returncurrent_2))))

(event `InputAxis|상하이동`
  (params (AxisValue :type "Float (single-precision)"))
  ;[1 1 1] 상하 선형보간 이동 기능
  (bind _returncurrent (`self.선형보간` (`self.CurrentZ`) AxisValue (/ (`self.SpeedMove`) 2.0)))
  (bind _output_get (set `self.CurrentZ` _returncurrent))
  (`self.K2_AddActorLocalOffset` (`KismetMathLibrary.MakeVector` 0.0 0.0 _output_get) true))

(event `InputAxis|회전`
  (params (AxisValue :type "Float (single-precision)"))
  ;[1 1 1] 좌우 선형보간 회전 기능
  (`|ExecutionSequence`
    (:`then_0`
      (bind _returncurrent (`self.선형보간` (`self.CurrentYaw`) AxisValue (`self.SpeedRot`)))
      (bind _output_get (set `self.CurrentYaw` _returncurrent))
      (`self.K2_AddActorLocalRotation` (`KismetMathLibrary.MakeRotator` 0.0 0.0 _output_get) true))
    (:`then_1`
      ;[1 1 1] 키보드와 마우스 회전 적용
      ;;[1 1 1] 회전시 SpringArm을 반대로 기울이기 값을 저장한다
      (bind _returncurrent_2 (`self.선형보간` (`self.ArmRoll`) AxisValue (`self.SpeedRoll`)))
      (set `self.ArmRoll` _returncurrent_2))))

(event `MouseUpDownEvent`
  (params (`Axis Value` :type "Float (double-precision)"))
  ;[1 1 1] 마우스 상하 선형보간 이동 기능
  (bind _returncurrent (`self.선형보간` (`self.CurrentZ`) `Axis Value` (`self.SpeedMove`)))
  (bind _output_get (set `self.CurrentZ` _returncurrent))
  (`self.K2_AddActorLocalOffset` (`KismetMathLibrary.MakeVector` 0.0 0.0 _output_get) true))

(event `InputAxis|마우스 상하회전`
  (params (AxisValue :type "Float (single-precision)"))
  ;[1 1 1] 키보드와 마우스 회전 적용
  ;;[1 1 1] 마우스 상하 회전 기능
  (`self.MouseUpDownEvent` AxisValue))

(event `InputAxis|마우스 좌우회전`
  (params (AxisValue :type "Float (single-precision)"))
  ;[1 1 1] 키보드와 마우스 회전 적용
  ;;[1 1 1] 마우스 좌우 회전 기능, 마우스좌우회전 입력축을 연결하면 Apache의 좌우를 볼 수 있다
  (`self.MouseLeftRightEvent` AxisValue))

(event `self.ReceiveTick`
  (params (DeltaSeconds :type "Float (single-precision)"))
  ;[1 1 1] 키보드와 마우스 회전 적용
  ;;[1 1 1] 키보드/마우스에서 변화시킨 값을 이곳에서 일괄 적용
  (`self.TickCheckEvent`)
  (`SceneComponent.K2_SetWorldRotation` (`self.SpringArm`) (`KismetMathLibrary.MakeRotator` (+ (`self.ArmRoll`) (.roll (`self.K2_GetActorRotation`))) (+ (`self.ArmPitch`) (.pitch (`self.K2_GetActorRotation`))) (+ (.yaw (`self.K2_GetActorRotation`)) (`self.ArmYaw`))) false false) ; 절대회전각도를 적용
)

(event `KillCountEvent`
  ;[1 1 1] 대공포가 파괴될 때마다 이벤트 수신
  (`KismetSystemLibrary.PrintString` (`KismetStringLibrary.Concat_StrStr` "KillCount = " (`KismetStringLibrary.Conv_IntToString` (`self.KillCount`)))))

(event `TickCheckEvent`
  ;[1 1 1] Tick이 발생할 때마다 이벤트 수신 후 처리
  (`self.SetFuel`)
  (`self.SetHP`)
  (`self.CheckComplete`))

(event `InputAction|발사`
  (params (Key :type "Key Structure"))
  (bind _spawnleft (`self.SpawnLeft`))
  (bind _spawnright (`self.SpawnRight`))
  ;[1 1 1] 발사 이벤트 시 좌우 로켓 생성
  (:`Pressed`
    (`|SpawnActorFromClass` "/Game/_01_ApacheEx/Blueprints/BP_ApacheRocket.BP_ApacheRocket_C" (`SceneComponent.K2_GetComponentToWorld` _spawnleft) "Undefined" "OverrideRootScale" null null)
    (`GameplayStatics.SpawnEmitterAtLocation` "/Game/_01_ApacheEx/Particles/P_Explosion2.P_Explosion2" (`SceneComponent.K2_GetComponentLocation` _spawnleft)))
  (:`Released`
    (`|SpawnActorFromClass` "/Game/_01_ApacheEx/Blueprints/BP_ApacheRocket.BP_ApacheRocket_C" (`SceneComponent.K2_GetComponentToWorld` _spawnright) "Undefined" "OverrideRootScale" null null)
    (`GameplayStatics.SpawnEmitterAtLocation` "/Game/_01_ApacheEx/Particles/P_Explosion2.P_Explosion2" (`SceneComponent.K2_GetComponentLocation` _spawnright))))

(event `self.Apache_Body.OnComponentHit`
  (params (HitComponent :type "PrimitiveComponent Object Reference") (OtherActor :type "Actor Object Reference") (OtherComp :type "PrimitiveComponent Object Reference") (NormalImpulse :type "Vector Structure") (Hit :type "HitResult Structure (by ref)"))
  ;[1 1 1] 아파치가 대공포에 피격되었을 때 처리
  (if (`self.ActorHasTag` OtherActor "TurretRocket")
    (`/Engine/EditorBlueprintResources/StandardMacros.DoOnce` false
      (:`Completed`
        (`self.DestroySelf`)))))

(event `self.ReceiveBeginPlay`
  (`UserWidget.AddToViewport` (`self.GameUI`) 0))

(event `InputAction|Popup Menu`
  (params (Key :type "Key Structure"))
  (:`Pressed`
    (set `self.IsPopUp` true)
    (`self.ShowPopUp`)))

(event `InputAction|1인칭/3인칭`
  (params (Key :type "Key Structure"))
  (bind _cockpit (`self.CockPit`))
  (bind _springarm (`self.SpringArm`))
  (:`Pressed`
    (`/Engine/EditorBlueprintResources/StandardMacros.FlipFlop`
      (:`A`
        (set `SpringArmComponent.TargetArmLength` -250.0 _springarm)
        (`UserWidget.AddToViewport` _cockpit 0))
      (:`B`
        (set `SpringArmComponent.TargetArmLength` 600.0 _springarm)
        (`Widget.RemoveFromParent` _cockpit)))))

(fn `AddFuel`
  (set `self.Fuel` (`KismetMathLibrary.FClamp` (+ (`self.Fuel`) 200.0) 0.0 (`self.FuelMax`))))

(fn `ChangeSound`
  (`AudioComponent.Stop` (`self.BGM`))
  (`AudioComponent.Stop` (`self.RotorSound`))
  (`AudioComponent.Play` (`self.Gameover`) 0.0))

(fn `CheckComplete`
  (if (>= (`self.KillCount`) (`self.EnemyCount`))
    (set `self.IsComplete` true)
    (`self.ShowsCursor` true)
    (`self.ShowMenu`)))

(fn `CreateUI`
  (`|ExecutionSequence`
    (:`then_0`
      (bind _returnvalue (`|CreateWidget` "/Game/_01_ApacheEx/UI/BP_GameUI.BP_GameUI_C"))
      (set `self.GameUI` _returnvalue))
    (:`then_1`
      (bind _returnvalue_2 (`|CreateWidget` "/Game/_01_ApacheEx/UI/BP_MainMenu.BP_MainMenu_C"))
      (set `self.MainMenu` _returnvalue_2))
    (:`then_2`
      (bind _returnvalue_3 (`|CreateWidget` "/Game/_01_ApacheEx/UI/BP_PopUpMenu.BP_PopUpMenu_C"))
      (set `self.PopUpMenu` _returnvalue_3))
    (:`then_3`
      (bind _returnvalue_4 (`|CreateWidget` "/Game/_01_ApacheEx/UI/BP_CockPit.BP_CockPit_C"))
      (set `self.CockPit` _returnvalue_4))))

(fn `DestroySelf`
  (bind _returnvalue (`self.K2_GetActorLocation`))
  (set `self.IsDead` true)
  (`GameplayStatics.SpawnEmitterAtLocation` "/Game/_01_ApacheEx/Particles/P_Explosion3.P_Explosion3" _returnvalue)
  (`GameplayStatics.PlaySoundAtLocation` "/Game/StarterContent/Audio/Explosion01.Explosion01" _returnvalue (struct) 1.0 1.0 0.0 null null null)
  (`self.SetDestroy`))

(fn `ScrollLeftRight`
  (params (AxisValue :type "Float (double-precision)"))
  (set `self.ArmYaw` (`KismetMathLibrary.FClamp` (+ AxisValue (`self.ArmYaw`)) -80.0 80.0)))

(fn `ScrollUpDown`
  (params (AxisValue :type "Float (double-precision)"))
  (set `self.ArmPitch` (`KismetMathLibrary.FClamp` (+ AxisValue (`self.ArmPitch`)) -30.0 80.0)))

(fn `SetDestroy`
  (`Widget.RemoveFromParent` (`self.CockPit`))
  (`self.SetActorHiddenInGame` true) ; 아파치를 숨긴다
  (`self.ChangeSound`)
  (`self.ShowsCursor` true)
  (`self.ShowMenu`))

(fn `SetFuel`
  ;[1 1 1] 게임 진행중
  (if (not (or (`self.IsDead`) (`self.IsComplete`) (`self.IsPopUp`)))
    (bind _output_get (set `self.Fuel` (- (`self.Fuel`) (* (`GameplayStatics.GetWorldDeltaSeconds`) 50.0))))
    (if (< _output_get 0.0)
      (`self.SetDestroy`))))

(fn `SetHP`
  (set `self.HP` (`KismetMathLibrary.FClamp` (/ (`self.Fuel`) (`self.FuelMax`)))))

(fn `SetMenuTitle`
  (if (`self.IsComplete`)
    (bind _returnvalue (`Image.GetDynamicMaterial` (`/Game/_01_ApacheEx/UI/BP_MainMenu.MenuTitle` (`self.MainMenu`))))
    (`MaterialInstanceDynamic.SetTextureParameterValue` _returnvalue "Title" "/Game/_01_ApacheEx/Textures/MissionComplete.MissionComplete")))

(fn `ShowMenu`
  (`/Engine/EditorBlueprintResources/StandardMacros.DoOnce` false
    (:`Completed`
      (`self.SetMenuTitle`)
      (`UserWidget.AddToViewport` (`self.MainMenu`) 0))))

(fn `ShowPopUp`
  (`UserWidget.AddToViewport` (`self.PopUpMenu`) 0)
  (`self.ShowsCursor` true))

(fn `ShowsCursor`
  (params (IsShow :type Boolean))
  (bind _returnvalue (`GameplayStatics.GetPlayerController` 0))
  (if IsShow
    ;[1 1 1] 게임상의 입력
    (`self.DisableInput` null)
    (else
      (`self.EnableInput` null)))
  ;[1 1 1] UI 메뉴의 커서와 클릭 이벤트 설정
  (set `PlayerController.bShowMouseCursor` IsShow _returnvalue)
  (set `PlayerController.bEnableClickEvents` IsShow _returnvalue))

(fn `UserConstructionScript`
  (`self.CreateUI`))

(fn `선형보간`
  (params (Current :type "Float (double-precision)") (`Axis Value` :type "Float (double-precision)") (Speed :type "Float (double-precision)"))
  (returns (ReturnCurrent :type "Float (double-precision)"))
  (bind _returnvalue (`GameplayStatics.GetWorldDeltaSeconds`))
  (return (`KismetMathLibrary.FInterpTo` Current (* `Axis Value` Speed _returnvalue) _returnvalue 4.0)))